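; BP_ButtonParent is a base Blueprint for world buttons that show their on or off state through colour.
; The construction script creates a dynamic material on the Button mesh, and activate and deactivate events set its ColourLerp parameter.
; ToggleActivate reads that parameter back as the state to pick which event to call.
; The Box overlap events are empty, so nothing in this graph triggers the button.
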(event OnComponentBeginOverlap(Box)
  (params (OverlappedComponent :type Primitive%20Component%20Object%20Reference) (OtherActor :type Actor%20Object%20Reference) (OtherComp :type Primitive%20Component%20Object%20Reference) (OtherBodyIndex :type Integer) (bFromSweep :type Boolean) (SweepResult :type Hit%20Result%20Structure%20%28by%20ref%29)))

(event OnComponentEndOverlap(Box)
  (params (OverlappedComponent :type Primitive%20Component%20Object%20Reference) (OtherActor :type Actor%20Object%20Reference) (OtherComp :type Primitive%20Component%20Object%20Reference) (OtherBodyIndex :type Integer)))

(event Custom|ButtonActivate
  ;[0.15 0.15 0.15 0.5] Activate
  (Rendering|Material|SetScalarParameterValue (Variables|Default|GetButtonMaterial) "ColourLerp" 1.0 :!class /Script/Engine.MaterialInstanceDynamic))

(event Custom|ButtonDeactivate
  ;[0.15 0.15 0.15 0.5] Deactivate
  (Rendering|Material|SetScalarParameterValue (Variables|Default|GetButtonMaterial) "ColourLerp" 0.0 :!class /Script/Engine.MaterialInstanceDynamic))

(event Custom|ToggleActivate
  ;[0.15 0.15 0.15 0.5] Toggle Button
  (bind _returnvalue (Rendering|Material|GetScalarParameterValue (Variables|Default|GetButtonMaterial) "ColourLerp" :!class /Script/Engine.MaterialInstanceDynamic))
  (if (== _returnvalue 0.0)
    (CallFunction|ButtonActivate)
    (else
      (CallFunction|ButtonDeactivate))))

(fn ConstructionScript
  (bind _returnvalue (Rendering|Material|CreateDynamicMaterialInstance (Variables|Default|GetButton) 0 0 "None" :!class /Script/Engine.PrimitiveComponent))
  (Variables|Default|SetButtonMaterial _returnvalue))