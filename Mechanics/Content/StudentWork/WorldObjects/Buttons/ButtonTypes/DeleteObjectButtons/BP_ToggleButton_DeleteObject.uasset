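; Toggle button Blueprint that swaps the static mesh of a target object, ObjectToChange, between active and deactive states.
; Activation sets the button material's ColourLerp parameter to its active value and applies ActiveMesh; deactivation reverses both with DeactiveMesh.
; The construction script runs the parent's setup, then applies DeactiveMesh so the object starts in its inactive look.
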(event EventButtonActivate
  ;[0.15 0.15 0.15 0.5] Activate
  (Rendering|Material|SetScalarParameterValue (Variables|Default|GetButtonMaterial) "ColourLerp" 1.0 :!class /Script/Engine.MaterialInstanceDynamic)
  (Components|StaticMesh|SetStaticMesh (Variables|Default|GetObjectToChange) (Variables|Default|GetActiveMesh)))

(event EventButtonDeactivate
  ;[0.15 0.15 0.15 0.5] Deactivate
  (Rendering|Material|SetScalarParameterValue (Variables|Default|GetButtonMaterial) "ColourLerp" 0.0 :!class /Script/Engine.MaterialInstanceDynamic)
  (Components|StaticMesh|SetStaticMesh (Variables|Default|GetObjectToChange) (Variables|Default|GetDeactiveMesh)))

(fn ConstructionScript
  (|CallParentFunction)
  (Components|StaticMesh|SetStaticMesh (Variables|Default|GetObjectToChange) (Variables|Default|GetDeactiveMesh)))