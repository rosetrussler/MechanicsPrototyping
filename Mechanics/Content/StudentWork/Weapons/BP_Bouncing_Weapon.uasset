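; BP_Bouncing_Weapon is a tank weapon that fires bouncing projectiles when triggered.
; Triggered spawns BP_Bouncing_Projectile at the location and rotation of the tank's DirectionArrow, unless the weapon is in cooldown.
; Each shot sets the InCooldown flag and starts a FireRate timer whose EndCooldown event clears it, so FireRate acts as the delay between shots.
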(event Custom|End%20Cooldown
  (Variables|Default|SetIn%20Cooldown false))

(event EventTriggered
  (bind _mytank (Variables|Default|GetMyTank))
  (bind _directionarrow (Variables|/Game/Blueprints/BP_PlayerCharacter.BP_PlayerCharacter_C|GetDirectionArrow _mytank))
  (if (not (Variables|Default|GetIn%20Cooldown)) ; If in cooldown
    (Game|SpawnActorfromClass "/Game/StudentWork/Weapons/Projectiles/BP_Bouncing_Projectile.BP_Bouncing_Projectile_C" (Math|Transform|MakeTransform (Transformation|GetWorldLocation _directionarrow) (Transformation|GetWorldRotation _directionarrow) "1.000000,1.000000,1.000000") "Undefined" "MultiplyWithRoot" 0 0)
    (Variables|Default|SetIn%20Cooldown true)
    (Utilities|Time|SetTimerbyEvent (delegate Custom|End%20Cooldown) (Variables|Default|GetFire%20Rate))))

(fn ConstructionScript
  (|CallParentFunction))