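; Enemy movement-type Blueprint that follows another enemy rather than choosing its own path.
; Its Move event uses AIMoveTo toward the stored enemy reference, or searches for a new target when that reference is invalid.
; The search takes the nearest other actor overlapping the detection sphere and stores it only if it is a BP_Enemy_Parent, otherwise printing a message.
; BeginPlay starts the movement and attack timers.
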(event Custom|FindNewTarget
  ;[0.15 0.15 0.15 0.5] Get target
  (bind _output_get (Variables|Default|SetOverlapping%20Actors (Collision|GetOverlappingActors (Variables|Default|GetDetection%20Sphere) 0 :!class /Script/Engine.PrimitiveComponent)))
  (Utilities|Array|RemoveItem _output_get self) ; Remove self from array
  (if (Utilities|Array|IsNotEmpty (Variables|Default|GetOverlapping%20Actors)) ; any enemy in radius?
    (bind _asbp_enemy_parent (Utilities|Casting|CastToBP_Enemy_Parent (.ReturnValue (Actor|FindNearestActor (Transformation|GetActorLocation) (Variables|Default|GetOverlapping%20Actors)))) ; find closest actor and check if enemy
      (:then
        (Variables|Default|SetEnemy%20Referance _asbp_enemy_parent))
      (:CastFailed
        (Development|PrintString "selected actor not enemy")))))

(event EventMove
  (bind _enemy_referance (Variables|Default|GetEnemy%20Referance))
  ;[0.15 0.15 0.15 0.5] Move
  (Utilities|IsValid _enemy_referance
    (:Is%20Valid
      (AI|AIMoveTo self "0, 0, 0" _enemy_referance (Variables|Default|GetAcceptance%20Radius) false))
    (:Is%20Not%20Valid
      (CallFunction|FindNewTarget))))

(event EventBeginPlay
  (CallFunction|StartMovementTimer)
  (CallFunction|StartAttackTimer))

(fn ConstructionScript
  (|CallParentFunction))