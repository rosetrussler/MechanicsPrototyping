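; Enemy movement-type Blueprint that sends the pawn along a looping list of waypoints.
; Move issues an AI MoveTo toward the current waypoint, provided the array is not empty.
; Both success and failure advance the index, wrapping to the first entry after the last, so unreachable points are skipped.
; The graph does not re-trigger Move itself, so each call covers a single leg.
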(event Custom|SwitchWaypoint
  ;[0.15 0.15 0.15 0.5] Switch waypoint
  (bind _output_get (Variables|Default|SetCurrent%20Waypoint%20Index (+ (Variables|Default|GetCurrent%20Waypoint%20Index) 1)))
  (if (> _output_get (Utilities|Array|LastIndex (Variables|Default|GetWaypointArray))) ; If index is greater than last item in array loop to start
    (Variables|Default|SetCurrent%20Waypoint%20Index 0)))

(event EventMove
  (if (not (== (Utilities|Array|LastIndex (Variables|Default|GetWaypointArray)) -1)) ; if something is in the array
    (AI|AIMoveTo self (Utilities|Array|Get(acopy) (Variables|Default|GetWaypointArray) (Variables|Default|GetCurrent%20Waypoint%20Index)) 0 5.0 false
      (:OnSuccess
        _)
      (:OnFail
        _))
    (CallFunction|SwitchWaypoint)))

(fn ConstructionScript
  (|CallParentFunction))