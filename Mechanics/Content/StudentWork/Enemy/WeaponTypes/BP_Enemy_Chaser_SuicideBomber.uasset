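; Suicide bomber variant of a chaser enemy that pursues the player and attacks once within bomb range.
; When the player character overlaps the detection sphere, it stores the reference and starts inherited movement and attack timers plus a colour timer.
; Attack fires the weapon at the player only if they are within BombDistance.
; The looping colour timer alternates two red emissive materials on the head for a flashing warning effect.
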(event OnComponentBeginOverlap(DetectionSphere)
  (params (OverlappedComponent :type Primitive%20Component%20Object%20Reference) (OtherActor :type Actor%20Object%20Reference) (OtherComp :type Primitive%20Component%20Object%20Reference) (OtherBodyIndex :type Integer) (bFromSweep :type Boolean) (SweepResult :type Hit%20Result%20Structure%20%28by%20ref%29))
  (bind _asbp_player_character (Utilities|Casting|CastToBP_PlayerCharacter OtherActor)) ; Is the pawn BP_PlayerCharecter?
  (Variables|Default|SetPlayer%20Referance _asbp_player_character) ; If cast is successful + store ref to player
  (CallFunction|StartMovementTimer)
  (CallFunction|StartAttackTimer)
  (CallFunction|StartColourTimer))

(event Custom|Switch%20Colours
  (if (== (Rendering|Material|GetMaterial (Variables|Default|GetHead) 1) "/Game/Materials/MI_EmissiveRed.MI_EmissiveRed") ; gets material and alternates for flashing effect
    (Rendering|Material|SetMaterial (Variables|Default|GetHead) 1 "/Game/Materials/MI_Emissive_Red_2.MI_Emissive_Red_2")
    (else
      (Rendering|Material|SetMaterial (Variables|Default|GetHead) 1 "/Game/Materials/MI_EmissiveRed.MI_EmissiveRed"))))

(event Custom|Start%20Colour%20Timer
  (bind _returnvalue (Utilities|Time|SetTimerbyEvent (delegate Custom|Switch%20Colours) (Variables|Default|GetTimeBetweenColours) true))
  (Variables|Default|SetColourTimer _returnvalue))

(event EventAttack
  (if (<= (Transformation|GetDistanceTo (Variables|Default|GetPlayer%20Referance)) (Variables|Default|GetBombDistance)) ; If in range
    (CallFunction|FireWeaponatActor (Variables|Default|GetPlayer%20Referance))))

(fn ConstructionScript
  (|CallParentFunction))