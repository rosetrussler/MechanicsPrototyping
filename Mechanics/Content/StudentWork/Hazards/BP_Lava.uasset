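; BP_Lava is a lava hazard that damages actors overlapping its static mesh.
; Begin overlap adds the actor to an array, deals damage immediately and sets a looping timer that damages every tracked actor.
; Each new overlap sets another timer and overwrites the single stored handle.
; End overlap removes valid actors and clears that stored timer once the array is empty.
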(event OnComponentBeginOverlap(StaticMesh)
  (params (OverlappedComponent :type Primitive%20Component%20Object%20Reference) (OtherActor :type Actor%20Object%20Reference) (OtherComp :type Primitive%20Component%20Object%20Reference) (OtherBodyIndex :type Integer) (bFromSweep :type Boolean) (SweepResult :type Hit%20Result%20Structure%20%28by%20ref%29))
  ;[0.15 0.15 0.15 0.5] Start of overlap
  (Utilities|Array|Add (Variables|Default|GetActors%20in%20lava) OtherActor) ; Add actor to array
  (Game|Damage|ApplyDamage OtherActor (Variables|Default|GetBase%20Damage) 0 0) ; Damages the pawn which is overlapping
  (bind _returnvalue (Utilities|Time|SetTimerbyEvent (delegate Custom|Apply%20Damage) (Variables|Default|GetTime%20Between%20Damage) true))
  (Variables|Default|SetLava%20Timer%20 _returnvalue))

(event OnComponentEndOverlap(StaticMesh)
  (params (OverlappedComponent :type Primitive%20Component%20Object%20Reference) (OtherActor :type Actor%20Object%20Reference) (OtherComp :type Primitive%20Component%20Object%20Reference) (OtherBodyIndex :type Integer))
  ;[0.15 0.15 0.15 0.5] End of overlap
  (Utilities|IsValid OtherActor ; If object is valid
    (:Is%20Valid
      (Utilities|Array|RemoveItem (Variables|Default|GetActors%20in%20lava) OtherActor) ; Remove from array
      (if (== (Utilities|Array|Length (Variables|Default|GetActors%20in%20lava)) 0) ; If nothing in arrray
        (Utilities|Time|ClearandInvalidateTimerbyHandle (Variables|Default|GetLava%20Timer%20)) ; End timer
      ))))

(event Custom|Apply%20Damage
  ;[0.15 0.15 0.15 0.5] Apply damage
  (for _array_element (Variables|Default|GetActors%20in%20lava)
    (Game|Damage|ApplyDamage _array_element (Variables|Default|GetBase%20Damage) 0 0) ; Damages the pawn which is overlapping
  ))

(fn ConstructionScript)