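; BP_EnemyTurret is an enemy turret hazard that fires projectiles on a fixed interval and can be destroyed by damage.
; On BeginPlay it starts a looping timer at FireRate that spawns BP_Enemy_Projectile at the Arrow component's world location and rotation.
; AnyDamage subtracts incoming damage from CurrentHealth and destroys the turret when health reaches zero or below.
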(event Custom|Fire%20Projectile
  (bind _arrow (Variables|Default|GetArrow))
  ;[0.15 0.15 0.15 0.5] Fire
  (Game|SpawnActorfromClass "/Game/StudentWork/Weapons/Projectiles/BP_Enemy_Projectile.BP_Enemy_Projectile_C" (Math|Transform|MakeTransform (Transformation|GetWorldLocation _arrow) (Transformation|GetWorldRotation _arrow) "1.000000,1.000000,1.000000") "Undefined" "MultiplyWithRoot" 0 0))

(event EventBeginPlay
  ;[0.15 0.15 0.15 0.5] Start Firing
  (bind _returnvalue (Utilities|Time|SetTimerbyEvent (delegate Custom|Fire%20Projectile) (Variables|Default|GetFire%20Rate) true))
  (Variables|Default|SetTurret%20Timer _returnvalue))

(event Game|Damage|EventAnyDamage
  (params (Damage :type Float%20%28single-precision%29) (DamageType :type Damage%20Type%20Object%20Reference) (InstigatedBy :type Controller%20Object%20Reference) (DamageCauser :type Actor%20Object%20Reference))
  ;[0.15 0.15 0.15 0.5] take damage
  (Variables|Default|SetCurrent%20Health (- (Variables|Default|GetCurrent%20Health) Damage)) ; apply damage
  (if (<= (Variables|Default|GetCurrent%20Health) 0.0) ; If health less than 0
    (Actor|DestroyActor) ; kill self
  ))

(fn ConstructionScript)