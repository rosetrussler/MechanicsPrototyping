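; BP_ExplosiveBarrel is an actor that flashes and then explodes the first time it takes any damage.
; The construction script creates a dynamic material instance on the mesh, and a timeline drives its FlashLevel parameter.
; When the flash finishes, it clears the mesh, activates the NSBigExplosion effect and applies radial damage within DamageRadius.
; It destroys itself after a short delay.
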(event Game|Damage|EventAnyDamage
  (params (Damage :type Float%20%28single-precision%29) (DamageType :type Damage%20Type%20Object%20Reference) (InstigatedBy :type Controller%20Object%20Reference) (DamageCauser :type Actor%20Object%20Reference))
  (Utilities|FlowControl|DoOnce false
    (:Completed
      (bind _flash (Timeline|Flash PlayFromStart)
        (:Update
          (Rendering|Material|SetScalarParameterValue (Variables|Default|GetFlash%20Material) "FlashLevel" _flash :!class /Script/Engine.MaterialInstanceDynamic))
        (:Finished
          (Components|StaticMesh|SetStaticMesh (Variables|Default|GetStaticMesh) 0)
          (Components|Activation|Activate (Variables|Default|GetNS_BigExplosion) false) ; Explode
          (Game|Damage|ApplyRadialDamage 1e+01 (Transformation|GetActorLocation) (Variables|Default|GetDamage%20Radius) 0 0 0 0 false "ECC_Visibility")
          (Utilities|FlowControl|Delay 1.0)
          (Actor|DestroyActor))))))

(fn ConstructionScript
  (bind _returnvalue (Rendering|Material|CreateDynamicMaterialInstance (Variables|Default|GetStaticMesh) 0 0 "None" :!class /Script/Engine.PrimitiveComponent))
  (Variables|Default|SetFlash%20Material _returnvalue))